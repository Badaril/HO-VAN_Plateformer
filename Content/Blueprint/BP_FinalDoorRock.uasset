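; Final rock door that slides open or closed on light toggles and sets the Level 3 unlock flag.
; Binds to the custom GameInstance's light-toggle event, then plays an open or close timeline based on UpdateRockDoorState, skipping close if already closed.
; Timeline updates offset the actor along X from its current location, so movement accumulates per tick.
; The GameInstance stores the closed flag and the unlock result, set when each timeline finishes.
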(event Custom|UpdateDoorState
  (bind _doorstate (Default|UpdateRockDoorState (Variables|Default|GetGameInstanceRef)))
  (if _doorstate
    (bind _alpha (Timeline|OpenDoor PlayFromStart)
      (:Update
        (CallFunction|OpenLastDoor _alpha))
      (:Finished
        (Variables|/Game/Blueprint/BP_CustomGameinstance.BP_CustomGameinstance_C|SetLevel3Unlocked (Variables|Default|GetGameInstanceRef) true)))
    (elif (not (Variables|/Game/Blueprint/BP_CustomGameinstance.BP_CustomGameinstance_C|GetDoorIsAlreadyClosed (Variables|Default|GetGameInstanceRef)))
      (bind _alpha_2 (Timeline|CloseDoor PlayFromStart)
        (:Update
          (CallFunction|CloseLastDoor _alpha_2))
        (:Finished
          (Variables|/Game/Blueprint/BP_CustomGameinstance.BP_CustomGameinstance_C|SetLevel3Unlocked (Variables|Default|GetGameInstanceRef) false))))))

(event EventBeginPlay
  (bind _asbp_custom_gameinstance (Utilities|Casting|CastToBP_CustomGameinstance (Game|GetGameInstance)))
  (bind _output_get (Variables|Default|SetGameInstanceRef _asbp_custom_gameinstance))
  (EventDispatchers|BindEventtoOnLightToggle _output_get (delegate Custom|UpdateDoorState)))

(event Collision|EventActorBeginOverlap
  (params (OtherActor :type Actor%20Object%20Reference)))

(event EventTick
  (params (DeltaSeconds :type Float%20%28single-precision%29)))

(fn ConstructionScript)

(fn OpenLastDoor
  (params (Alpha :type Float%20%28double-precision%29))
  (bind _returnvalue (Transformation|GetActorLocation))
  (Transformation|SetActorLocation (Math|Interpolation|Ease "Linear" Alpha _returnvalue (+ _returnvalue "5.000000,0.000000,0.000000")) false false)
  (Variables|/Game/Blueprint/BP_CustomGameinstance.BP_CustomGameinstance_C|SetDoorIsAlreadyClosed (Variables|Default|GetGameInstanceRef) false))

(fn CloseLastDoor
  (params (Alpha :type Float%20%28double-precision%29))
  (bind _returnvalue (Transformation|GetActorLocation))
  (Transformation|SetActorLocation (Math|Interpolation|Ease "Linear" Alpha _returnvalue (- _returnvalue "5.000000,0.000000,0.000000")) false false)
  (Variables|/Game/Blueprint/BP_CustomGameinstance.BP_CustomGameinstance_C|SetDoorIsAlreadyClosed (Variables|Default|GetGameInstanceRef) true))