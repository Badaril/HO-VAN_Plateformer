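; BP_CollectibleBouton is a collectible button pickup that the player obtains when its Activate event fires.
; Activate sets HasPickedTheButton on the game instance, destroys the actor, then writes a congratulatory DialogueText saying the player can return to the surface.
; BeginPlay, overlap and Tick are disabled stubs, and nothing in the graphs shown assigns GameInstanceRef.
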(event EventBeginPlay
  (|CallParentFunction) ; This node is disabled and will not be called.\nDrag off pins to build functionality.
)

(event Collision|EventActorBeginOverlap
  (params (OtherActor :type Actor%20Object%20Reference))
  (|CallParentFunction OtherActor) ; This node is disabled and will not be called.\nDrag off pins to build functionality.
)

(event EventTick
  (params (DeltaSeconds :type Float%20%28single-precision%29))
  (|CallParentFunction DeltaSeconds) ; This node is disabled and will not be called.\nDrag off pins to build functionality.
)

(event EventActivate
  (Variables|/Game/Blueprint/BP_CustomGameinstance.BP_CustomGameinstance_C|SetHasPickedTheButton (Variables|Default|GetGameInstanceRef) true)
  (Actor|DestroyActor)
  (Variables|/Game/Blueprint/BP_CustomGameinstance.BP_CustomGameinstance_C|SetDialogueText (Variables|Default|GetGameInstanceRef) "You've got the button, congratulations. You can come back to the surface. "))

(fn ConstructionScript
  (|CallParentFunction))