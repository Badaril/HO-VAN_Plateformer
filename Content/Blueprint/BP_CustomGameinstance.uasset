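; Custom Game Instance that holds shared state for a light-toggle door puzzle and the player's health (PV).
; UpdateLight flips the lights at the given indices and calls OnLightToggle, while UpdateDoorState returns true only when every light checked is on.
; UpdatePVPlayer adds the Damage value to health within a small clamped range.
; CheckGameProgression is unfinished: its below-zero check leads nowhere, and the pause-and-widget logic is disconnected.
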(fn UpdateLight
  (params (ListOfLightsControlled :type Array%20of%20Integers))
  (bind _listoflights (Variables|Default|GetListOfLights))
  (for _array_element ListOfLightsControlled
    (Utilities|Array|SetArrayElem _listoflights _array_element (not (Utilities|Array|Get(acopy) _listoflights _array_element))))
  (Default|CallOnLightToggle))

(fn GetLightStatebyIndex
  (params (IndexLight :type Integer))
  (return (Utilities|Array|Get(acopy) (Variables|Default|GetListOfLights) IndexLight)))

(fn UpdateDoorState
  (bind _array_element (Utilities|Array|ForEachLoopwithBreak (Variables|Default|GetListOfLights) :!label _label)
    (:LoopBody
      (bind _output_get (LocalVariables|SetTempDoorState _array_element))
      (if (not _output_get)
        (goto _label Break)))
    (:Completed
      (return (LocalVariables|GetTempDoorState)))))

(fn UpdatePVPlayer
  (params (Damage :type Integer))
  (Variables|Default|SetPVPlayer (Math|Integer|Clamp(Integer) (+ Damage (Variables|Default|GetPVPlayer)) 0 3)))

(fn CheckGameProgression
  (if (< (Variables|Default|GetPVPlayer) 0)
    _))