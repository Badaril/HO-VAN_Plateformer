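; BP_Light is a light actor whose point light visibility follows a per-index on/off state stored in the custom game instance.
; On BeginPlay it caches BP_CustomGameinstance, binds ChangeLight to that instance's OnLightToggle event and runs it once to set the initial state.
; ChangeLight looks up the state for the actor's Index and applies it to the PointLight's visibility.
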(event Custom|ChangeLight
  (bind _lightstate (Default|GetLightStatebyIndex (Variables|Default|GetGameInstanceRef) (Variables|Default|GetIndex)))
  (Rendering|SetVisibility (Variables|Default|GetPointLight) _lightstate false))

(event EventBeginPlay
  (bind _asbp_custom_gameinstance (Utilities|Casting|CastToBP_CustomGameinstance (Game|GetGameInstance)))
  (bind _output_get (Variables|Default|SetGameInstanceRef _asbp_custom_gameinstance))
  (EventDispatchers|BindEventtoOnLightToggle _output_get (delegate Custom|ChangeLight))
  (CallFunction|ChangeLight))

(event Collision|EventActorBeginOverlap
  (params (OtherActor :type Actor%20Object%20Reference)))

(event EventTick
  (params (DeltaSeconds :type Float%20%28single-precision%29)))

(fn ConstructionScript)