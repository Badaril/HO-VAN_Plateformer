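; BP_Door is a door that opens only when the score stored in BP_CustomGameinstance reaches a threshold.
; BeginPlay caches the game instance, and the Activate event checks its score.
; On success, the OpenDoor timeline linearly eases the door's world rotation to a 90-degree turn.
; On failure, a second timeline eases it from that turn back to zero while writing a refusal message to the game instance's dialogue text.
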(event EventBeginPlay
  (bind _asbp_custom_gameinstance (Utilities|Casting|CastToBP_CustomGameinstance (Game|GetGameInstance)))
  (Variables|Default|SetGameInstanceRef _asbp_custom_gameinstance))

(event Collision|EventActorBeginOverlap
  (params (OtherActor :type Actor%20Object%20Reference)))

(event EventTick
  (params (DeltaSeconds :type Float%20%28single-precision%29)))

(event EventActivate
  (if (>= (Variables|/Game/Blueprint/BP_CustomGameinstance.BP_CustomGameinstance_C|GetScore (Variables|Default|GetGameInstanceRef)) 100)
    (bind _alpha (Timeline|OpenDoor PlayFromStart)
      (:Update
        (Transformation|SetWorldRotation (Variables|Default|GetDoor) (Math|Interpolation|Ease :Function "Linear" :Alpha _alpha :B "0.000000,90.000000,0.000000") false false)))
    (else
      (bind _alpha_2 (Timeline|Timeline PlayFromStart)
        (:Update
          (Transformation|SetWorldRotation (Variables|Default|GetDoor) (Math|Interpolation|Ease :Function "Linear" :Alpha _alpha_2 :A "0.000000,90.000000,0.000000") false false)
          (Variables|/Game/Blueprint/BP_CustomGameinstance.BP_CustomGameinstance_C|SetDialogueText (Variables|Default|GetGameInstanceRef) "You cannot pass. You need 100 score to open the door."))))))

(fn ConstructionScript)