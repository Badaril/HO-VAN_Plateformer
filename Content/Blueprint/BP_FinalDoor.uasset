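; BP_FinalDoor is the last door, with two mesh panels that swing open or closed based on game instance state.
; On BeginPlay it binds to the game instance's OnLightToggle, then queries UpdateDoorState on each call to pick the open or close timeline.
; The timelines drive each panel toward fixed world rotations, easing from its current rotation every update, so placed actor rotation is ignored.
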(event Custom|UpdateDoorState
  (bind _doorstate (Default|UpdateDoorState (Variables|Default|GetGameInstanceRef)))
  (if _doorstate
    (bind _alpha (Timeline|OpenDoor PlayFromStart)
      (:Update
        (CallFunction|OpenLastDoor _alpha)))
    (else
      (bind _alpha_2 (Timeline|Timeline PlayFromStart)
        (:Update
          (CallFunction|CloseLastDoor _alpha_2))))))

(event EventBeginPlay
  (bind _asbp_custom_gameinstance (Utilities|Casting|CastToBP_CustomGameinstance (Game|GetGameInstance)))
  (bind _output_get (Variables|Default|SetGameInstanceRef _asbp_custom_gameinstance))
  (EventDispatchers|BindEventtoOnLightToggle _output_get (delegate Custom|UpdateDoorState)))

(event Collision|EventActorBeginOverlap
  (params (OtherActor :type Actor%20Object%20Reference)))

(event EventTick
  (params (DeltaSeconds :type Float%20%28single-precision%29)))

(fn ConstructionScript)

(fn OpenLastDoor
  (params (Alpha :type Float%20%28double-precision%29))
  (Transformation|SetWorldRotation (Variables|Default|GetStaticMesh1) (Math|Interpolation|Ease "Linear" Alpha (Transformation|GetWorldRotation (Variables|Default|GetStaticMesh1)) "0.000000,-90.000000,0.000000" true) false false)
  (Transformation|SetWorldRotation (Variables|Default|GetStaticMesh) (Math|Interpolation|Ease "Linear" Alpha (Transformation|GetWorldRotation (Variables|Default|GetStaticMesh)) "0.000000,-90.000000,0.000000" true) false false))

(fn CloseLastDoor
  (params (Alpha :type Float%20%28double-precision%29))
  (Transformation|SetWorldRotation (Variables|Default|GetStaticMesh1) (Math|Interpolation|Ease "Linear" Alpha (Transformation|GetWorldRotation (Variables|Default|GetStaticMesh1)) "0.000000,0.000000,0.000000" true) false false)
  (Transformation|SetWorldRotation (Variables|Default|GetStaticMesh) (Math|Interpolation|Ease "Linear" Alpha (Transformation|GetWorldRotation (Variables|Default|GetStaticMesh)) "0.000000,-180.000000,0.000000" true) false false))