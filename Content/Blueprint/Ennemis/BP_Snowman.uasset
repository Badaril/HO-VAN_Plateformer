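; Snowman enemy that patrols back and forth along world X and can be destroyed by a running player.
; Timelines chain through the Move event to loop walking and 180-degree turns.
; Each walk update offsets from the current location, so movement accumulates rather than interpolating between fixed endpoints.
; Player overlap plays a pop sound; if the player is running, it spawns a BP_Carrot overhead and destroys itself.
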(event Custom|Move
  (params (Direction :type Boolean))
  (if Direction
    (bind _alpha (Timeline|MoveForward PlayFromStart)
      (:Update
        (CallFunction|Walking _alpha))
      (:Finished
        (bind _alpha_2 (Timeline|Timeline_1 PlayFromStart)
          (:Update
            (Transformation|SetActorRotation (Math|Interpolation|Ease :Function "Linear" :Alpha _alpha_2 :B "0.000000,180.000000,0.000000")))
          (:Finished
            (CallFunction|Move false)))))
    (else
      (bind _alpha_3 (Timeline|MoveBack PlayFromStart)
        (:Update
          (CallFunction|WalkingBack _alpha_3))
        (:Finished
          (bind _alpha_4 (Timeline|Timeline_2 PlayFromStart)
            (:Update
              (Transformation|SetActorRotation (Math|Interpolation|Ease :Function "Linear" :Alpha _alpha_4 :A "0.000000,180.000000,0.000000")))
            (:Finished
              (CallFunction|Move true))))))))

(event EventBeginPlay
  (CallFunction|Move true))

(event Collision|EventActorBeginOverlap
  (params (OtherActor :type Actor%20Object%20Reference))
  (bind _asbp_player (Utilities|Casting|CastToBP_Player OtherActor))
  (Audio|PlaySound2D "/Game/Sounds/PopSound.PopSound" 0.1 0.2 0.0 0 0)
  (if (Variables|/Game/Blueprint/PlayerCharacter/BP_Player.BP_Player_C|GetRunning _asbp_player)
    (Game|SpawnActorfromClass "/Game/Blueprint/Ennemis/BP_Carrot.BP_Carrot_C" (Math|Transform|MakeTransform (+ (Transformation|GetWorldLocation (Variables|Default|GetDefaultSceneRoot)) "0.000000,0.000000,400.000000") "0, 0, 0" "1.000000,1.000000,1.000000") "Undefined" "MultiplyWithRoot" 0 0)
    (Utilities|FlowControl|Delay 0.0)
    (Actor|DestroyActor)))

(fn ConstructionScript)

(fn Walking
  (params (Alpha :type Float%20%28single-precision%29))
  (bind _returnvalue (Transformation|GetActorLocation))
  (Transformation|SetActorLocation (Math|Interpolation|Ease "Linear" Alpha _returnvalue (+ _returnvalue (Math|Vector|MakeVector (Variables|Default|GetDistance) 0.0 0.0))) false false))

(fn WalkingBack
  (params (Alpha :type Float%20%28double-precision%29))
  (bind _returnvalue (Transformation|GetActorLocation))
  (Transformation|SetActorLocation (Math|Interpolation|Ease "Linear" Alpha _returnvalue (- _returnvalue (Math|Vector|MakeVector (Variables|Default|GetDistance) 0.0 0.0))) false false))