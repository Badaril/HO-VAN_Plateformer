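; BP_ShootingSnowman is a stationary snowman enemy that fires snowballs and can be destroyed by a running player.
; From BeginPlay, a self-repeating Shoot event spawns a snowball at the Arrow component with a sound, destroys it after a short delay, then fires again.
; Player overlap always plays a pop sound, but only a running player makes it spawn a carrot above itself and destroy itself.
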(event Custom|Shoot
  (bind _arrow (Variables|Default|GetArrow))
  (bind _returnvalue (Transformation|GetWorldLocation _arrow))
  (bind _returnvalue_2 (+ _returnvalue "10.000000,0.000000,0.000000"))
  (bind _returnvalue_3 (Game|SpawnActorfromClass "/Game/Blueprint/Ennemis/BP_Snowball.BP_Snowball_C" (Math|Transform|MakeTransform _returnvalue_2 "0, 0, 0" "1.000000,1.000000,1.000000") "Undefined" "MultiplyWithRoot" 0 0))
  (Audio|PlaySoundatLocation "/Game/Sounds/SW_Shooting.SW_Shooting" _returnvalue_2 "0, 0, 0" 0.1 1.0 0.5 0 0 0 0)
  (bind _output_get (Variables|Default|SetSnowball _returnvalue_3))
  (Utilities|FlowControl|Delay 2.0)
  (Actor|DestroyActor _output_get)
  (CallFunction|Shoot))

(event EventBeginPlay
  (CallFunction|Shoot))

(event Collision|EventActorBeginOverlap
  (params (OtherActor :type Actor%20Object%20Reference))
  (bind _asbp_player (Utilities|Casting|CastToBP_Player OtherActor))
  (Audio|PlaySound2D "/Game/Sounds/PopSound.PopSound" 0.1 0.2 0.0 0 0)
  (if (Variables|/Game/Blueprint/PlayerCharacter/BP_Player.BP_Player_C|GetRunning _asbp_player)
    (Game|SpawnActorfromClass "/Game/Blueprint/Ennemis/BP_Carrot.BP_Carrot_C" (Math|Transform|MakeTransform (+ (Transformation|GetWorldLocation (Variables|Default|GetDefaultSceneRoot)) "0.000000,0.000000,400.000000") "0, 0, 0" "1.000000,1.000000,1.000000") "Undefined" "MultiplyWithRoot" 0 0)
    (Utilities|FlowControl|Delay 0.0)
    (Actor|DestroyActor)))

(fn ConstructionScript)